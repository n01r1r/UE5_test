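; BP_AssetManager is a test manager actor that opens a media source on a MediaPlayer when play begins.
; BeginPlay switches on MediaSourceID, with three cases each calling OpenSource.
; It reads VideoID from the MPC_test parameter collection, but the truncation into MediaSourceID is disconnected, so that value never selects the case.
; The construction script collects all BP_MeshTest actors into MeshesToControl, which nothing here uses.
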(event `self.ReceiveBeginPlay`
  (bind _returnvalue (`KismetMaterialLibrary.GetScalarParameterValue` "/Game/Movies/MPC_test.MPC_test" "VideoID"))
  (switch `int` (`self.MediaSourceID`)
    (:`0`
      (`MediaPlayer.OpenSource` (`self.MediaPlayer`) null))
    (:`1`
      (`MediaPlayer.OpenSource` (`self.MediaPlayer`) null))
    (:`2`
      (`MediaPlayer.OpenSource` (`self.MediaPlayer`) null))))

(fn `UserConstructionScript`
  (bind _outactors (`GameplayStatics.GetAllActorsOfClass` "/Game/Movies/BP_MeshTest.BP_MeshTest_C"))
  (for _array_element _outactors
    (`KismetArrayLibrary.Array_Add` (`self.MeshesToControl`) _array_element)))