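; BP_MeshTest is a clickable mesh actor, apparently a video screen, that opens a media selection menu.
; On BeginPlay it writes UV offsets, UV divisions and a video ID into the static mesh's custom primitive data, allowing per-instance variation without separate materials.
; Clicking the mesh creates a WB_MediaSelection widget for the first player controller and adds it to the viewport.
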(event `self.ReceiveBeginPlay`
  (bind _staticmesh (`self.StaticMesh`))
  ;[1 1 1] U[0], V[1] Offset
  (`PrimitiveComponent.SetCustomPrimitiveDataFloat` _staticmesh 0 (`self.UOffset`))
  (`PrimitiveComponent.SetCustomPrimitiveDataFloat` _staticmesh 1 (`self.VOffset`))
  ;[1 1 1] U Divide[2], V Divide[3]
  (`PrimitiveComponent.SetCustomPrimitiveDataFloat` _staticmesh 2 (`self.UDiv`))
  (`PrimitiveComponent.SetCustomPrimitiveDataFloat` _staticmesh 3 (`self.VDiv`))
  (`PrimitiveComponent.SetCustomPrimitiveDataFloat` (`self.StaticMesh`) 4 (`self.VideoID`)))

(event `self.StaticMesh.OnClicked`
  (params (TouchedComponent :type "PrimitiveComponent Object Reference") (ButtonPressed :type "Key Structure"))
  ;[1 1 1] Show Widget
  (bind _returnvalue (`|CreateWidget` "/Game/Movies/WB_MediaSelection.WB_MediaSelection_C" (`GameplayStatics.GetPlayerController` 0)))
  (bind _output_get (set `self.WidgetVar` _returnvalue))
  (`UserWidget.AddToViewport` _output_get 0))

(fn `UserConstructionScript`)